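; BP_Drifter is an enemy ice platform that slides along its Y axis and carries the player who lands on it.
; On BeginPlay it caches the IceBlast_BP player and runs a timeline that lerps IceMesh toward EndLocationCube, then destroys itself.
; Box overlap snaps an unattached player to the mesh's Top socket and notifies it.
; Either DeathBox overlapping the player tells the game mode to end the game.
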(event OnComponentBeginOverlap(Box)
  (params (OverlappedComponent :type Primitive%20Component%20Object%20Reference) (OtherActor :type Actor%20Object%20Reference) (OtherComp :type Primitive%20Component%20Object%20Reference) (OtherBodyIndex :type Integer) (bFromSweep :type Boolean) (SweepResult :type Hit%20Result%20Structure%20%28by%20ref%29))
  (bind _player_ (Class|BPIPlayerChar|IsPlayerCharacter(Message) OtherActor))
  (bind _isattached (Class|BPIPlayerChar|AttachReturn(Message) OtherActor))
  (if (and (not _isattached) _player_)
    (Transformation|AttachComponentToComponent (Variables|Default|GetPlayer) (Variables|Default|GetIceMesh) "Top" "SnapToTarget" "SnapToTarget" "KeepWorld" true)
    (CallFunction|ActorRotation)
    (Class|BPIPlayerChar|Attach(Message) (Variables|Default|GetPlayer) true)))

(event OnComponentBeginOverlap(DeathBox)
  (params (OverlappedComponent :type Primitive%20Component%20Object%20Reference) (OtherActor :type Actor%20Object%20Reference) (OtherComp :type Primitive%20Component%20Object%20Reference) (OtherBodyIndex :type Integer) (bFromSweep :type Boolean) (SweepResult :type Hit%20Result%20Structure%20%28by%20ref%29))
  (bind _player_ (Class|BPIPlayerChar|IsPlayerCharacter(Message) OtherActor))
  (if _player_
    (Class|BPIGameMode|EndGame(Message) (Game|GetGameMode))))

(event OnComponentBeginOverlap(DeathBox2)
  (params (OverlappedComponent :type Primitive%20Component%20Object%20Reference) (OtherActor :type Actor%20Object%20Reference) (OtherComp :type Primitive%20Component%20Object%20Reference) (OtherBodyIndex :type Integer) (bFromSweep :type Boolean) (SweepResult :type Hit%20Result%20Structure%20%28by%20ref%29))
  (bind _player_ (Class|BPIPlayerChar|IsPlayerCharacter(Message) OtherActor))
  (if _player_
    (Class|BPIGameMode|EndGame(Message) (Game|GetGameMode))))

(event Custom|DrifterSlide
  (bind _icemesh (Variables|Default|GetIceMesh))
  (bind _relativelocation (Variables|/Script/Engine.SceneComponent|GetRelativeLocation _icemesh))
  (bind _slide (Timeline|Slide PlayFromStart)
    (:Update
      (Transformation|SetRelativeLocation (Variables|Default|GetIceMesh) (Math|Vector|Lerp(Vector) (Variables|/Script/Engine.SceneComponent|GetRelativeLocation _icemesh) (Math|Vector|MakeVector (.x _relativelocation) (Variables|Default|GetEnd%20Location%20Cube) (.z _relativelocation)) _slide) false false))
    (:Finished
      (Actor|DestroyActor))))

(event EventBeginPlay
  (CallFunction|PlayerReference)
  (CallFunction|DrifterSlide))

(fn ConstructionScript)

(fn ActorRotation)

(fn PlayerReference
  (bind _returnvalue (Actor|GetActorOfClass "/Game/Blueprints/IceCharacter/IceBlast_BP.IceBlast_BP_C"))
  (Variables|Default|SetPlayer _returnvalue))

(fn IsEnemy?
  (return true))

(fn ReturnIceSickle
  (return false))