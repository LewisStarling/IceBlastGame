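; BP_DrifterSpawner is an enemy spawner that periodically creates BP_Drifter actors at its root location.
; A looping timer started on BeginPlay runs Spawn Drifter, which stores each new instance as CurrentDrifter.
; A DespawnBox, positioned from DespawnLocation in the construction script, destroys an overlapping actor only if it is the most recently spawned Drifter.
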(event OnComponentBeginOverlap(DespawnBox)
  (params (OverlappedComponent :type Primitive%20Component%20Object%20Reference) (OtherActor :type Actor%20Object%20Reference) (OtherComp :type Primitive%20Component%20Object%20Reference) (OtherBodyIndex :type Integer) (bFromSweep :type Boolean) (SweepResult :type Hit%20Result%20Structure%20%28by%20ref%29))
  (if (== OtherActor (Variables|Default|GetCurrentDrifter))
    (Actor|DestroyActor (Variables|Default|GetCurrentDrifter))))

(event EventBeginPlay
  (Utilities|Time|SetTimerbyFunctionName 0 "Spawn Drifter" 3.0 true))

(fn ConstructionScript
  (Transformation|SetRelativeLocation (Variables|Default|GetDespawnBox) (Variables|Default|GetDespawnLocation) false false))

(fn SpawnDrifter
  (bind _returnvalue (Game|SpawnActorfromClass "/Game/Blueprints/Enemies/Drifter/BP_Drifter.BP_Drifter_C" (Math|Transform|MakeTransform (Transformation|GetWorldLocation (Variables|Default|GetDefaultSceneRoot)) "0, 0, 0" "1,1,1") "AdjustIfPossibleButAlwaysSpawn" 0 0))
  (Variables|Default|SetCurrentDrifter _returnvalue))