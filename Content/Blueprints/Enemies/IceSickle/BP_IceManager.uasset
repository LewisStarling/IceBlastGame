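; BP_IceManager is an icicle hazard manager that drops a group of IceSickle actors when the player enters its trigger.
; StartBox overlap uses an IsPlayerCharacterMessage interface check, then calls Drop on every valid entry in IceSickles.
; The construction script sizes StartBox to the Cube's X scale with fixed Y and Z, and positions it at BoxLocation.
; BeginPlay records each icicle's location in IceLocations, which these graphs never read.
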(event OnComponentBeginOverlap(StartBox)
  (params (OverlappedComponent :type Primitive%20Component%20Object%20Reference) (OtherActor :type Actor%20Object%20Reference) (OtherComp :type Primitive%20Component%20Object%20Reference) (OtherBodyIndex :type Integer) (bFromSweep :type Boolean) (SweepResult :type Hit%20Result%20Structure%20%28by%20ref%29))
  (bind _player_ (Class|BPIPlayerChar|IsPlayerCharacter(Message) OtherActor))
  (if _player_
    (for _array_element (Variables|Default|GetIceSickles)
      (Utilities|IsValid _array_element
        (:Is%20Valid
          (Default|Drop _array_element))))))

(event EventBeginPlay
  (for _array_element (Variables|Default|GetIceSickles)
    (Utilities|Array|Add (Variables|Default|GetIce%20Locations) (Transformation|GetActorLocation _array_element))))

(fn ConstructionScript
  (Transformation|SetRelativeScale3D (Variables|Default|GetStart%20Box) (Math|Vector|MakeVector (.x (Variables|/Script/Engine.SceneComponent|GetRelativeScale3D (Variables|Default|GetCube))) 2.0 1.5))
  (Transformation|SetRelativeLocation (Variables|Default|GetStart%20Box) (Variables|Default|GetBox%20Location) false false))