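; Icicle hazard enemy that falls under physics and ends the game through the game mode when it overlaps the player.
; BeginPlay caches the start location and creates a dynamic ice material; the random drop-time assignment is disconnected.
; Drop, not called within this Blueprint, waits DropTime, simulates physics briefly, fades the material, then teleports back to start.
; Query functions identify it as an enemy icicle and return its home location.
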(event OnComponentBeginOverlap(icicle)
  (params (OverlappedComponent :type Primitive%20Component%20Object%20Reference) (OtherActor :type Actor%20Object%20Reference) (OtherComp :type Primitive%20Component%20Object%20Reference) (OtherBodyIndex :type Integer) (bFromSweep :type Boolean) (SweepResult :type Hit%20Result%20Structure%20%28by%20ref%29))
  (bind _player_ (Class|BPIPlayerChar|IsPlayerCharacter(Message) OtherActor))
  (if _player_
    (Class|BPIGameMode|EndGame(Message) (Game|GetGameMode))
    (Transformation|Teleport (Variables|Default|GetDefault%20Location) "0, 0, 0")))

(event Custom|Drop
  (Utilities|FlowControl|RetriggerableDelay (Variables|Default|GetDrop%20Time))
  (Physics|SetSimulatePhysics (Variables|Default|Geticicle) true)
  (Utilities|FlowControl|Delay 1.0)
  (CallFunction|MaterialFade)
  (Physics|SetSimulatePhysics (Variables|Default|Geticicle) false))

(event Custom|InitChain
  (Variables|Default|SetDefault%20Location (Transformation|GetActorLocation))
  (CallFunction|CreateMaterialInstance)
  (CallFunction|SetActorDefaultLocation)
  (CallFunction|SetRandomDropTime))

(event Custom|Material%20Fade
  (bind _materialfade (Timeline|FadeOut PlayFromStart)
    (:Update
      (Rendering|Material|SetScalarParameterValue (Variables|Default|GetMI_Ice) "Fade" (Math|Float|Lerp 1.0 0.0 _materialfade) :!class /Script/Engine.MaterialInstanceDynamic))
    (:Finished
      (Rendering|Material|SetScalarParameterValue (Variables|Default|GetMI_Ice) "Fade" 1.0 :!class /Script/Engine.MaterialInstanceDynamic)
      (Physics|SetSimulatePhysics (Variables|Default|Geticicle) false)
      (Transformation|Teleport (Variables|Default|GetDefault%20Location) "0, 0, 0"))))

(event EventBeginPlay
  (CallFunction|InitChain))

(fn ConstructionScript)

(fn CreateMaterialInstance
  (bind _returnvalue (Rendering|Material|CreateDynamicMaterialInstance (Variables|Default|Geticicle) 0 "/Game/Assets/Materials/M_Ice.M_Ice" "None" :!class /Script/Engine.PrimitiveComponent))
  (Variables|Default|SetMI_Ice _returnvalue))

(fn SetActorDefaultLocation
  (Variables|Default|SetDefault%20Location (Transformation|GetActorLocation)))

(fn SetRandomDropTime)

(fn IsEnemy?
  (return true))

(fn ReturnIceSickle
  (return true (Variables|Default|GetDefault%20Location)))