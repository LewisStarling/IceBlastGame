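; IceBlast_BP is an ice player character that can attach to other actors and launch off them.
; Releasing Jump detaches it and, if it was attached, calls SetSideForce, applies a velocity impulse to Ice, then clears Attached after a short delay.
; A fast looping timer treats near-zero vertical velocity as landing.
; BoundsCheck, not called here, also teleports the actor onto a fixed X plane.
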(event Custom|KeepingPlayerInBounds
  (if (Math|Float|InRange(Float) (.z (Transformation|GetVelocity)) -0.4 0.3)
    (Class|IceBlastPawn|OnLanded)))

(event EventBeginPlay
  (Utilities|Time|SetTimerbyEvent (delegate Custom|KeepingPlayerInBounds) 0.01 true))

(event EventAttach
  (params (Attached :type Boolean))
  (Variables|Default|SetAttached Attached))

(event Input|ActionEvents|InputActionJump
  (params (Key :type Key%20Structure :default "None"))
  (:Released
    (Transformation|DetachFromActor "KeepWorld" "KeepRelative" "KeepWorld")
    (if (Variables|Default|GetAttached)
      (Class|IceBlastPawn|SetSideForce)
      (Physics|AddImpulse (Variables|Default|GetIce) (Variables|Default|GetAdded%20Velocity_0) "None" true)
      (Utilities|FlowControl|Delay 0.2)
      (Variables|Default|SetAttached false))))

(fn ConstructionScript)

(fn BoundsCheck
  (bind _returnvalue (Transformation|GetActorLocation))
  (Transformation|Teleport (Math|Vector|MakeVector 1205.0 (.y _returnvalue) (.z _returnvalue)) "0, 0, 0")
  (if (Math|Float|InRange(Float) (.z (Transformation|GetVelocity)) -0.4 0.3)
    (Class|IceBlastPawn|OnLanded)))

(fn AttachReturn
  (return (Variables|Default|GetAttached)))

(fn IsPlayerCharacter
  (return true))