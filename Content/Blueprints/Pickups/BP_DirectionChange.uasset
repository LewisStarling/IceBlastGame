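; Pickup that launches the IceBlast_BP player in the direction their DashArrow points.
; On player overlap it hides itself, shows the arrow and slows global time for a brief, dilation-stretched delay.
; It then applies a velocity-change impulse to the player's Ice component, restores time and hides the arrow.
; A Reset flag blocks retriggering until the pickup reappears after a cooldown; the visibility helper also prints a debug string.
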(event Collision|EventActorBeginOverlap
  (params (OtherActor :type Actor%20Object%20Reference))
  (bind _player (Variables|Default|GetPlayer))
  (bind _player_ (Class|BPIPlayerChar|IsPlayerCharacter(Message) OtherActor))
  (if _player_
    (if (Variables|Default|Getreset%20)
      (Variables|Default|Setreset%20 false)
      (CallFunction|SetVisibilty true false)
      (Utilities|Time|SetGlobalTimeDilation 0.1)
      (Utilities|FlowControl|Delay 0.2)
      (Physics|AddImpulse (Variables|/Script/IceBlastGame.IceBlastPawn|GetIce _player) (* (Math|Rotator|GetRotationXVector (Transformation|GetWorldRotation (Variables|/Game/Blueprints/IceCharacter/IceBlast_BP.IceBlast_BP_C|GetDash%20Arrow _player))) 9e+02) "None" true)
      (Utilities|Time|SetGlobalTimeDilation 1.0)
      (CallFunction|SetVisibilty true true)
      (Utilities|FlowControl|Delay 5.0)
      (CallFunction|SetVisibilty false true)
      (Variables|Default|Setreset%20 true))))

(event EventBeginPlay
  (bind _returnvalue (Actor|GetActorOfClass "/Game/Blueprints/IceCharacter/IceBlast_BP.IceBlast_BP_C"))
  (Variables|Default|SetPlayer _returnvalue))

(fn ConstructionScript)

(fn SetVisibilty
  (params (This%20pickup%20Hidden :type Boolean) (Arrow%20Hidden :type Boolean))
  (bind _returnvalue (not Arrow%20Hidden))
  (Rendering|SetActorHiddenInGame This%20pickup%20Hidden)
  (Development|PrintString (Utilities|String|ToString(Boolean) _returnvalue))
  (Rendering|SetVisibility (Variables|/Game/Blueprints/IceCharacter/IceBlast_BP.IceBlast_BP_C|GetDash%20Arrow (Variables|Default|GetPlayer)) _returnvalue false))