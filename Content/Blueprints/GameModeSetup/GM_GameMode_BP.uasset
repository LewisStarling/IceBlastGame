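; GM_GameMode_BP is a game mode that manages respawning for the IceBlast_BP player.
; On BeginPlay it caches the player and all BP_RespawnPoint actors, selecting index 0 as the active point.
; ChangeRespawn switches the active point by Index, and EndGame teleports the player to it.
; EndGame then briefly enables collision on that point's four MovemetomStop components, apparently to kill leftover momentum.
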(event EventBeginPlay
  (bind _returnvalue (Actor|GetActorOfClass "/Game/Blueprints/IceCharacter/IceBlast_BP.IceBlast_BP_C"))
  (Variables|Default|SetIce%20Player%20 _returnvalue)
  (bind _outactors (Actor|GetAllActorsOfClass "/Game/Blueprints/GameModeSetup/BP_RespawnPoint.BP_RespawnPoint_C"))
  (bind _output_get (Variables|Default|SetRespawnPoints _outactors))
  (for _array_element _output_get
    (if (== (Variables|/Game/Blueprints/GameModeSetup/BP_RespawnPoint.BP_RespawnPoint_C|GetIndex _array_element) 0)
      (Variables|Default|SetRespawn%20Point%20 _array_element))))

(event EventChangeRespawn
  (params (Index :type Integer))
  (for _array_element (Variables|Default|GetRespawnPoints)
    (if (== (Variables|/Game/Blueprints/GameModeSetup/BP_RespawnPoint.BP_RespawnPoint_C|GetIndex _array_element) Index)
      (Variables|Default|SetRespawn%20Point%20 _array_element))))

(event EventEndGame
  (Transformation|SetActorLocation (Variables|Default|GetIce%20Player%20) (Transformation|GetActorLocation (Variables|Default|GetRespawn%20Point%20)) false true)
  (Collision|SetCollisionEnabled (Variables|/Game/Blueprints/GameModeSetup/BP_RespawnPoint.BP_RespawnPoint_C|GetMovemetom%20stop%20 (Variables|Default|GetRespawn%20Point%20)) "QueryAndPhysics")
  (Utilities|FlowControl|Delay 0.1)
  (Collision|SetCollisionEnabled (Variables|/Game/Blueprints/GameModeSetup/BP_RespawnPoint.BP_RespawnPoint_C|GetMovemetom%20stop%20 (Variables|Default|GetRespawn%20Point%20)) "NoCollision"))

(fn ConstructionScript)